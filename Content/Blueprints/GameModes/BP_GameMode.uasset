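; BP_GameMode is a game mode that sets up VR display on start and keeps counts of collectables.
; BeginPlay runs console commands for fullscreen, stereo rendering and HMD mirror mode.
; SetTotalCollectables and SetCollectableCount add the passed value to their counters rather than overwrite them.
; Collected lowers the current count by one through SetCollectableCount, with no completion check here.
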(event Custom|SetTotalCollectables
  (params (Value :type Integer))
  (Variables|Default|SetTotalCollectables (+ (Variables|Default|GetTotalCollectables) Value)))

(event Custom|SetCollectableCount
  (params (Value :type Integer))
  (Variables|Default|SetCollectableCount (+ Value (Variables|Default|GetCollectableCount))))

(event EventBeginPlay
  (Development|ExecuteConsoleCommand "FULLSCREEN")
  (Development|ExecuteConsoleCommand "Stereo On")
  (Development|ExecuteConsoleCommand "HMD mirror mode 4"))

(event EventCollected
  (CallFunction|SetCollectableCount -1))

(fn ConstructionScript)