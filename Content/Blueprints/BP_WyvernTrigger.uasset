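; BP_WyvernTrigger is a trigger volume that fires a wyvern spawn when the player enters it.
; On box overlap by a BP_Player, it calls SpawnItem on its WyvernSpawner reference, then sets HasSpawned so the spawn happens only once.
; The construction script sets the box extent from ColliderScale, so the trigger area is sized through that variable.
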(event OnComponentBeginOverlap(Box)
  (params (OverlappedComponent :type Primitive%20Component%20Object%20Reference) (OtherActor :type Actor%20Object%20Reference) (OtherComp :type Primitive%20Component%20Object%20Reference) (OtherBodyIndex :type Integer) (bFromSweep :type Boolean) (SweepResult :type Hit%20Result%20Structure%20%28by%20ref%29))
  (Utilities|Casting|CastToBP_Player OtherActor)
  (if (not (Variables|Default|GetbHasSpawned))
    (Default|SpawnItem (Variables|Default|GetWyvernSpawner))
    (Variables|Default|SetbHasSpawned true)))

(fn ConstructionScript
  (Components|Box|SetBoxExtent (Variables|Default|GetBox) (Variables|Default|GetColliderScale) true))