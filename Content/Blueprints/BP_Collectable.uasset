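; Collectable pickup that homes in on the player and is collected on touch.
; Box overlap stores the player, after which Tick blends ProjectileMovement velocity halfway toward the player's direction at Speed each frame, staying still until then.
; Sphere overlap calls Collected, passes -1 to the GameMode's SetTotalCollectables, plays a sound and destroys the actor.
; BeginPlay caches the GameMode and sets its CollectableCount to 1.
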(event OnComponentBeginOverlap(Box)
  (params (OverlappedComponent :type Primitive%20Component%20Object%20Reference) (OtherActor :type Actor%20Object%20Reference) (OtherComp :type Primitive%20Component%20Object%20Reference) (OtherBodyIndex :type Integer) (bFromSweep :type Boolean) (SweepResult :type Hit%20Result%20Structure%20%28by%20ref%29))
  (bind _asbp_player (Utilities|Casting|CastToBP_Player OtherActor))
  (Utilities|IsValid (Variables|Default|GetBPPlayer)
    (:Is%20Not%20Valid
      (Variables|Default|SetBPPlayer _asbp_player))))

(event OnComponentBeginOverlap(Sphere)
  (params (OverlappedComponent :type Primitive%20Component%20Object%20Reference) (OtherActor :type Actor%20Object%20Reference) (OtherComp :type Primitive%20Component%20Object%20Reference) (OtherBodyIndex :type Integer) (bFromSweep :type Boolean) (SweepResult :type Hit%20Result%20Structure%20%28by%20ref%29))
  (Utilities|Casting|CastToBP_Player OtherActor)
  (CallFunction|Collected)
  (Default|SetTotalCollectables (Variables|Default|GetBP_GameMode) -1)
  (Audio|PlaySoundatLocation "/Game/Assets/Audio/ui_menu_button_scroll_back_07.ui_menu_button_scroll_back_07" (Transformation|GetActorLocation))
  (Actor|DestroyActor))

(event EventTick
  (params (DeltaSeconds :type Float%20%28single-precision%29))
  (bind _projectilemovement (Variables|Default|GetProjectileMovement))
  (Utilities|IsValid (Variables|Default|GetBPPlayer)
    (:Is%20Valid
      (Variables|/Script/Engine.MovementComponent|SetVelocity _projectilemovement (Math|Vector|Lerp(Vector) (Variables|/Script/Engine.MovementComponent|GetVelocity (Variables|Default|GetProjectileMovement)) (* (Math|Vector|Normalize (- (Transformation|GetActorLocation (Variables|Default|GetBPPlayer)) (Transformation|GetActorLocation))) (Variables|Default|GetSpeed)) 0.5)))
    (:Is%20Not%20Valid
      (Variables|/Script/Engine.MovementComponent|SetVelocity _projectilemovement "0.000000, 0, 0"))))

(event EventBeginPlay
  (bind _asbp_game_mode (Utilities|Casting|CastToBP_GameMode (Game|GetGameMode)))
  (bind _output_get (Variables|Default|SetBP_GameMode _asbp_game_mode))
  (Variables|/Game/Blueprints/GameModes/BP_GameMode.BP_GameMode_C|SetCollectableCount _output_get 1))

(fn ConstructionScript)