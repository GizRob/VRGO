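; BP_Wyvern is a flying enemy that rises on spawn, keeps facing the VR player and ragdolls when killed.
; A BeginPlay timeline lifts it toward a fixed height, while Tick turns it toward the player's VROrigin.
; SpitFire aims an arrow component at the player and spawns BP_ProjectileEnemy, but nothing here calls it; the FireAtPlayer timer is disconnected.
; Damage depletes Health, then enables mesh physics and destroys the actor after a delay.
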(event Custom|FireAtPlayer)

(event Custom|SpitFire
  (bind _arrow (Variables|Default|GetArrow))
  (Transformation|SetWorldRotation _arrow (Math|Rotator|FindLookatRotation (Transformation|GetWorldLocation _arrow) (Transformation|GetWorldLocation (Variables|/Game/Blueprints/Player/BP_Player.BP_Player_C|GetVROrigin (Variables|Default|GetBP_Player)))) false false)
  (Game|SpawnActorfromClass "/Game/Blueprints/BP_ProjectileEnemy.BP_ProjectileEnemy_C" (Transformation|GetWorldTransform (Variables|Default|GetArrow)) "AlwaysSpawn" 0 0))

(event Game|Damage|EventAnyDamage
  (params (Damage :type Float%20%28single-precision%29) (DamageType :type Damage%20Type%20Object%20Reference) (InstigatedBy :type Controller%20Object%20Reference) (DamageCauser :type Actor%20Object%20Reference))
  (bind _output_get (Variables|Default|SetHealth (- (Variables|Default|GetHealth) Damage)))
  (if (<= _output_get 0.0)
    (Variables|Default|SetbIsDead true)
    (Physics|SetSimulatePhysics (Variables|Default|GetSkeletalMesh) true)
    (Utilities|FlowControl|Delay 5.0)
    (Actor|DestroyActor)))

(event EventTick
  (params (DeltaSeconds :type Float%20%28single-precision%29))
  (Transformation|SetActorRotation (Math|Rotator|FindLookatRotation (Transformation|GetActorLocation) (Transformation|GetWorldLocation (Variables|/Game/Blueprints/Player/BP_Player.BP_Player_C|GetVROrigin (Variables|Default|GetBP_Player))))))

(event EventBeginPlay
  (bind _returnvalue (Transformation|GetActorLocation))
  (bind (_x _y) (Math|Vector|BreakVector _returnvalue))
  (bind _asbp_player (Utilities|Casting|CastToBP_Player (Game|Player|GetPlayerPawn 0)))
  (Variables|Default|SetBP_Player _asbp_player)
  (bind _newtrack_0 (Timeline|SpawnAnimation Play)
    (:Update
      (Transformation|SetActorLocation (Math|Vector|Lerp(Vector) _returnvalue (Math|Vector|MakeVector _x _y 7e+02) (* _newtrack_0 (Utilities|Time|GetWorldDeltaSeconds))) false false))
    (:Finished
      (Variables|Default|SetbIsRising false))))

(fn ConstructionScript)