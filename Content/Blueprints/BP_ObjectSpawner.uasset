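; Spawner actor that places an instance of a configurable Object class at its own transform, registering collectables with the game mode.
; On BeginPlay it caches BP_GameMode and runs SpawnItem if AutoSpawn is set; SpawnItem is also a standalone event.
; SpawnItem always spawns regardless of collision, with itself as owner, then calls SetTotalCollectables on the game mode if Object casts to BP_Collectable.
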(event Custom|SpawnItem
  (bind _object (Variables|Default|GetObject))
  (Game|SpawnActorfromClass _object (Transformation|GetActorTransform) "AlwaysSpawn" self 0)
  (Utilities|Casting|CastToBP_CollectableClass _object)
  (Default|SetTotalCollectables (Variables|Default|GetGameMode) 1))

(event EventBeginPlay
  (bind _asbp_game_mode (Utilities|Casting|CastToBP_GameMode (Game|GetGameMode)))
  (Variables|Default|SetGameMode _asbp_game_mode)
  (if (Variables|Default|GetbAutoSpawn)
    (CallFunction|SpawnItem)))

(fn ConstructionScript)