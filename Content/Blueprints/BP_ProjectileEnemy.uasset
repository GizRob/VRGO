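; Enemy projectile actor that damages what it touches and then destroys itself.
; A whoosh sound plays at its location on spawn.
; An overlap on its sphere applies generic damage, while a blocking hit applies point damage with the hit info and plays a flame ignite sound.
; Neither path filters the other actor, and only the hit path has an impact sound.
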(event OnComponentBeginOverlap(Sphere)
  (params (OverlappedComponent :type Primitive%20Component%20Object%20Reference) (OtherActor :type Actor%20Object%20Reference) (OtherComp :type Primitive%20Component%20Object%20Reference) (OtherBodyIndex :type Integer) (bFromSweep :type Boolean) (SweepResult :type Hit%20Result%20Structure%20%28by%20ref%29))
  (Game|Damage|ApplyDamage OtherActor 1.0 0 0 "/Script/Engine.DamageType")
  (Actor|DestroyActor))

(event Collision|EventHit
  (params (MyComp :type Primitive%20Component%20Object%20Reference) (Other :type Actor%20Object%20Reference) (OtherComp :type Primitive%20Component%20Object%20Reference) (bSelfMoved :type Boolean) (HitLocation :type Vector :default "0, 0, 0") (HitNormal :type Vector :default "0, 0, 0") (NormalImpulse :type Vector :default "0, 0, 0") (Hit :type Hit%20Result%20Structure%20%28by%20ref%29))
  (Game|Damage|ApplyPointDamage Other 1.0 (.ImpactPoint (Collision|BreakHitResult Hit)) Hit 0 self "/Script/Engine.DamageType")
  (Audio|PlaySoundatLocation "/Game/Assets/Audio/gas_large_flame_ignite_01.gas_large_flame_ignite_01" (Transformation|GetActorLocation))
  (Actor|DestroyActor))

(event EventBeginPlay
  (Audio|PlaySoundatLocation "/Game/Assets/Audio/whoosh_slow_deep_12.whoosh_slow_deep_12" (Transformation|GetActorLocation)))

(fn ConstructionScript)