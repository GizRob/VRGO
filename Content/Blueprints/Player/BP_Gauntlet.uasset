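; BP_Gauntlet is a rotating pickup that snaps to the player's interactor and shoots fireballs with hand feedback.
; Pickup stops the spin and disables physics, and pressing pickup again with the same interactor fires instead of dropping.
; Firing spawns BP_Projectile_Fireball at FirePoint only when the game mode's TotalCollectables is zero.
; A Dropped timer respawns it through its owning spawner, but its only call here sits in unreachable drop logic.
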(event Custom|SetRotationSpeed
  (params (Rate :type Rotator))
  (Variables|/Script/Engine.RotatingMovementComponent|SetRotationRate (Variables|Default|GetRotatingMovement) Rate))

(event Custom|Dropped
  (Timeline|DroppedCounter Play
    (:Finished
      (bind _asbp_object_spawner (Utilities|Casting|CastToBP_ObjectSpawner (Components|GetOwner)))
      (Default|SpawnItem _asbp_object_spawner)
      (Actor|DestroyActor))))

(event Custom|Picked
  (Timeline|DroppedCounter Stop
    (:Finished
      (bind _asbp_object_spawner (Utilities|Casting|CastToBP_ObjectSpawner (Components|GetOwner)))
      (Default|SpawnItem _asbp_object_spawner)
      (Actor|DestroyActor))))

(event EventBeginPlay
  (bind _asbp_game_mode (Utilities|Casting|CastToBP_GameMode (Game|GetGameMode)))
  (Variables|Default|SetBP_GameMode _asbp_game_mode)
  (Variables|Default|SetLocation (Transformation|GetActorLocation))
  (Variables|Default|SetStartTransform (Transformation|GetActorTransform))
  (CallFunction|SetRotationSpeed "0, 0,180.000000"))

(fn ConstructionScript)

(fn GetClosestPointandPriority
  (params (Interactor :type BPC%20World%20Interactor%20Object%20Reference))
  (return (.OutPointOnBody (Collision|GetClosestPointonCollision (Variables|Default|GetGauntlet) (Transformation|GetWorldLocation Interactor) "None")) 0))

(fn OnDrag
  (params (Interactor :type BPC%20World%20Interactor%20Object%20Reference))
  (return false))

(fn OnDragStart
  (params (Interactor :type BPC%20World%20Interactor%20Object%20Reference))
  (return false))

(fn OnDragStop
  (params (Interactor :type BPC%20World%20Interactor%20Object%20Reference))
  (return false))

(fn OnHover
  (params (Interactor :type BPC%20World%20Interactor%20Object%20Reference)))

(fn OnPickupPressed
  (params (Interactor :type BPC%20World%20Interactor%20Object%20Reference))
  (if (and (== (Variables|Default|GetInteractor) Interactor) (Utilities|IsValid (Variables|Default|GetInteractor))) ; If Pickup Pressed again with the same interactor drop otherwise pickup
    (CallFunction|OnUsePressed Interactor)
    (else
      ;[1 1 1] Pickup
      (Variables|Default|SetInteractor Interactor)
      (CallFunction|SetRotationSpeed "0, 0, 0")
      (Physics|SetSimulatePhysics (Variables|Default|GetGauntlet) false)
      (Transformation|AttachComponentToComponent (Variables|Default|GetInteractor) "None" "SnapToTarget" "SnapToTarget" "KeepWorld" true)
      (CallFunction|Picked)))
  (return false))

(fn OnPickupReleased
  (params (Interactor :type BPC%20World%20Interactor%20Object%20Reference))
  (return false))

(fn OnUnhover
  (params (Interactor :type BPC%20World%20Interactor%20Object%20Reference)))

(fn OnUsePressed
  (params (Interactor :type BPC%20World%20Interactor%20Object%20Reference))
  (bind _firepoint (Variables|Default|GetFirePoint))
  (bind _returnvalue (Transformation|GetWorldTransform _firepoint))
  (if (== (Variables|/Game/Blueprints/GameModes/BP_GameMode.BP_GameMode_C|GetTotalCollectables (Variables|Default|GetBP_GameMode)) 0)
    ;[1 1 1] Spawn bullet
    (bind _returnvalue_2 (Game|SpawnActorfromClass "/Game/Blueprints/BP_Projectile_Fireball.BP_Projectile_Fireball_C" (Math|Transform|MakeTransform (.location _returnvalue) (.rotation _returnvalue) "0.500000,0.500000,0.500000") "AlwaysSpawn" 0 0))
    (Actor|SetLifeSpan _returnvalue_2 1e+01)
    (Utilities|IsValid (Variables|Default|GetInteractor)
      (:Is%20Valid
        (CallFunction|PlayFeedbackonHand (Default|GetHand (Variables|Default|GetInteractor)) "NewEnumerator0" "NewEnumerator1" (Game|GetPlayerController 0)))
      (:Is%20Not%20Valid
        _))
    (return false)))

(fn OnUseReleased
  (params (Interactor :type BPC%20World%20Interactor%20Object%20Reference))
  (return false))